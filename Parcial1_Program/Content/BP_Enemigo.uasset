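; BP_Enemigo is an enemy actor that moves on its own and can fire bullets.
; Every Tick it adds its Speed as a local offset without sweep or delta-time scaling.
; BeginPlay sets a timer on a custom event that, while Shooting is true, calls SpawnBala to spawn a BP_Bala at the enemy's location, passing BulletSpeed as its Speed.
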(event `self.ReceiveTick`
  (params (DeltaSeconds :type "Float (single-precision)"))
  (`self.K2_AddActorLocalOffset` (`self.Speed`)))

(event `self.ReceiveBeginPlay`
  (`KismetSystemLibrary.K2_SetTimerDelegate` (delegate `CustomEvent`)))

(event `CustomEvent`
  (if (`self.Shooting`)
    (`self.Spawn Bala`)))

(fn `Spawn Bala`
  (`|SpawnActorFromClass` "/Game/BP_Bala.BP_Bala_C" (`KismetMathLibrary.MakeTransform` (`self.K2_GetActorLocation`)) "Undefined" "MultiplyWithRoot" null (`self.Bullet Speed`) null))

(fn `UserConstructionScript`)